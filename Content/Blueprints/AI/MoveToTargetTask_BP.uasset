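; Behavior tree task that moves the AI pawn toward the TargetToFollow blackboard actor every tick, with no finish call.
; It feeds a flattened, frame-time-scaled direction into WallSlideMove rather than using navigation pathfinding.
; It then yaws the scene component stored in SightLocRot to face the target, printing a debug string if the target is invalid.
; An older swept AddActorWorldOffset move remains disconnected.
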(event EventReceiveTickAI
  (params (OwnerController :type AI%20Controller%20Object%20Reference) (ControlledPawn :type Pawn%20Object%20Reference) (DeltaSeconds :type Float%20%28single-precision%29))
  (bind _returnvalue (Transformation|GetActorLocation ControlledPawn))
  (bind _targettofollow (Variables|Default|GetTargetToFollow))
  (bind _returnvalue_2 (AI|BehaviorTree|GetBlackboardValueasActor _targettofollow))
  (bind _returnvalue_3 (Transformation|GetActorLocation _returnvalue_2))
  (Utilities|IsValid _returnvalue_2
    (:Is%20Valid
      (Class|UnitBlueprintLibrary|WallSlideMove ControlledPawn (* (Math|Vector|Normalize (* (- _returnvalue_3 _returnvalue) "1.000000,1.000000, 0")) (* 1.3e+02 (Utilities|Time|GetWorldDeltaSeconds))) 65.0)
      (bind _asscene_component (Utilities|Casting|CastToSceneComponent (Class|BTFunctionLibrary|GetBlackboardValueasObject (Variables|Default|GetSightLocRot))))
      (Transformation|SetWorldRotation _asscene_component (Math|Rotator|MakeRotator 0.0 0.0 (.yaw (Math|Rotator|FindLookatRotation _returnvalue _returnvalue_3))) false false) ; Look
    )
    (:Is%20Not%20Valid
      (Development|PrintString "WHY"))))