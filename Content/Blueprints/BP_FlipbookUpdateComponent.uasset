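; Helper component for Paper2D flipbook sprites that face the camera and change art with viewing direction.
; LookAtCamera yaws an arrow component toward the camera and tilts the flipbook by control pitch.
; GetAngleNumber wraps the yaw between target facing and camera view into 45-degree sectors.
; SetFlipbookByAngleNum maps that sector to NorthWest or SouthWest art, mirroring via negative X scale for the opposite side, and keeps it playing.
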(event EventBeginPlay)

(event EventTick
  (params (DeltaSeconds :type Float%20%28single-precision%29)))

(fn LookatCamera
  (params (ArrowComp :type Scene%20Component%20Object%20Reference) (FlipbookComp :type Scene%20Component%20Object%20Reference))
  (bind _returnvalue (Game|GetPlayerCameraManager 0))
  (Utilities|IsValid _returnvalue
    (:Is%20Valid
      (Transformation|SetRelativeRotation ArrowComp (Math|Rotator|MakeRotator 0.0 0.0 (- (.yaw (Math|Rotator|FindLookatRotation (Transformation|GetWorldLocation ArrowComp) (Camera|GetCameraLocation _returnvalue))) 9e+01)) false false) ; Rotate Arrow
      (Transformation|SetRelativeRotation FlipbookComp (Math|Rotator|MakeRotator (.pitch (Pawn|GetControlRotation (Game|GetPlayerController 0) :!class /Script/Engine.Controller)) 0.0 0.0) false false) ; Rotate Flipbook
    )))

(fn GetAngleNumber
  (params (TargetLocation :type Vector) (TargetLookingRot :type Float%20%28single-precision%29) (Debug :type Boolean))
  (bind _returnvalue (Game|GetPlayerCameraManager 0))
  (bind _returnvalue_2 (Camera|GetCameraLocation _returnvalue))
  (bind _returnvalue_3 (Math|Rotator|FindLookatRotation _returnvalue_2 TargetLocation))
  (bind _returnvalue_4 (- TargetLookingRot (.yaw _returnvalue_3)))
  (bind _returnvalue_5 (> _returnvalue_4 1.8e+02))
  (bind _returnvalue_6 (- _returnvalue_4 3.6e+02))
  (bind _returnvalue_7 (Math|Float|SelectFloat _returnvalue_6 _returnvalue_4 _returnvalue_5))
  (bind _returnvalue_8 (< _returnvalue_7 -1.8e+02))
  (bind _returnvalue_9 (+ _returnvalue_7 3.6e+02))
  (bind _returnvalue_10 (Math|Float|SelectFloat _returnvalue_9 _returnvalue_7 _returnvalue_8))
  (bind _returnvalue_11 (/ _returnvalue_10 45.0))
  (bind _returnvalue_12 (Math|Float|Floor _returnvalue_11))
  (Development|PrintString (Utilities|String|ToString(Integer) _returnvalue_12) Debug Debug)
  (return _returnvalue_12))

(fn SetFlipbookbyAngleNum
  (params (DirFlipbooks :type Direction%20Flipbooks%20Structure) (AngleNum :type Integer) (FlipbookComp :type Paper%20Flipbook%20Component%20Object%20Reference))
  (bind (_southwest _northwest) (Utilities|Struct|BreakDirectionFlipbooks DirFlipbooks))
  (bind (_southwest_2 _northwest_2 _loop) (Utilities|Struct|BreakDirectionFlipbooks DirFlipbooks))
  (switch int AngleNum
    (:Default
      (Development|PrintString "Unexpected AngleNum " true true "(R=1.000000,G=0.000000,B=0.512609,A=1.000000)"))
    (:-4
      (Sprite|SetFlipbook FlipbookComp _southwest_2 :!label _label)
      (Transformation|SetWorldScale3D FlipbookComp "1.000000,1.000000,1.000000" :!label _label_2)
      (Components|Timeline|SetLooping FlipbookComp _loop :!label _label_3)
      (if (not (Audio|Components|Audio|IsPlaying FlipbookComp))
        (Audio|Components|Audio|Play FlipbookComp)))
    (:-3
      (goto _label))
    (:-2
      (goto _label))
    (:-1
      (Sprite|SetFlipbook FlipbookComp _northwest_2)
      (goto _label_2))
    (:0
      (Sprite|SetFlipbook FlipbookComp _northwest)
      (Transformation|SetWorldScale3D FlipbookComp "-1.000000,1.000000,1.000000" :!label _label_4)
      (goto _label_3))
    (:1
      (Sprite|SetFlipbook FlipbookComp _southwest :!label _label_5)
      (goto _label_4))
    (:2
      (goto _label_5))
    (:3
      (goto _label_5))))