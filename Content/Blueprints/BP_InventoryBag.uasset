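; Inventory bag that holds the item slots and owns the on-screen inventory UI.
; On BeginPlay it sizes the slot array, builds a UI_Inventory widget, passes itself to its action and item-info panels, then hides it.
; Show and Hide toggle the widget and switch input mode, with Show focusing the first slot; UpdateInventorySlot refreshes one slot by index.
; An unconnected chain for a UI_InventoryMainWidget variant never runs.
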(event EventBeginPlay
  (bind _self self)
  (Utilities|Array|Resize (Variables|Default|GetItemSlots) (Variables|Default|GetAmountOfSlots))
  (bind _returnvalue (UserInterface|CreateWidget "/Game/Blueprints/Widgets/UI_Inventory.UI_Inventory_C" 0 self (Variables|Default|GetSlotsPerRow)))
  (bind _output_get (Variables|Default|SetInventoryWidget _returnvalue))
  (Default|GenerateInventorySlots _output_get)
  (Variables|/Game/Blueprints/Widgets/UI_InventoryAction.UI_InventoryAction_C|SetInventoryBagRef (Variables|/Game/Blueprints/Widgets/UI_Inventory.UI_Inventory_C|GetUI_InventoryAction _output_get) _self)
  (Variables|/Game/Blueprints/Widgets/UI_InventoryItemInfo.UI_InventoryItemInfo_C|SetInventoryBagRef (Variables|/Game/Blueprints/Widgets/UI_Inventory.UI_Inventory_C|GetUI_InventoryItemInfo _output_get) _self)
  (UserInterface|Viewport|AddtoViewport _output_get 0)
  (CallFunction|HideInventory))

(event EventUpdateInventorySlot
  (params (EmptySlotIndex :type Integer))
  ;[1 1 1] Update Inventory Slot
  (Default|UpdateSlot (Utilities|Array|Get(acopy) (Variables|/Game/Blueprints/Widgets/UI_Inventory.UI_Inventory_C|GetInventorySlotWidgets (Variables|Default|GetInventoryWidget)) EmptySlotIndex)))

(fn ConstructionScript)

(fn ShowInventory
  (bind _inventorywidget (Variables|Default|GetInventoryWidget))
  (Widget|SetVisibility _inventorywidget "Visible")
  (Widget|SetIsEnabled _inventorywidget true)
  (bind _asbp_vvplayer_controller (Utilities|Casting|CastToBP_VVPlayerController (Game|GetPlayerController 0)))
  (Input|SetInputModeGameandUI _asbp_vvplayer_controller 0 "DoNotLock" true)
  (Default|SetFocusonSlot _inventorywidget))

(fn HideInventory
  (bind _inventorywidget (Variables|Default|GetInventoryWidget))
  (Widget|SetVisibility _inventorywidget "Hidden")
  (Widget|SetIsEnabled _inventorywidget false)
  (bind _asbp_vvplayer_controller (Utilities|Casting|CastToBP_VVPlayerController (Game|GetPlayerController 0)))
  (Input|SetInputModeGameOnly _asbp_vvplayer_controller))