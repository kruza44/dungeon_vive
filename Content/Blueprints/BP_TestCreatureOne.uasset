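; BP_TestCreatureOne is a test creature drawn as a directional flipbook sprite, with a perception meter widget.
; Each tick, FlipbookUpdateComponent turns the flipbook toward the camera and picks the CurrentAnimation frame set from the TargetDirection angle, with a debug arrow.
; A looping timer copies the PerceptionSphere's test string into the widget.
; Damage passes to the parent, and an angle-change check is left unconnected, so the flipbook is set every tick.
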(event Custom|SetPerceptionStateUI
  ;[1 1 1] SetPerceptionStateUI
  (Variables|/Game/Blueprints/Widgets/PerceptionStateWidget.PerceptionStateWidget_C|SetPerceptionMeter (.AsPerception%20State%20Widget (Utilities|Casting|CastToPerceptionStateWidget (UserInterface|GetUserWidgetObject (Variables|Default|GetPerceptionStateWidget)))) (Variables|/Script/Vive.PerceptionSphere|GetTestHUDString (Variables|Default|GetPerceptionSphere))))

(event EventBeginPlay
  (Utilities|Time|SetTimerbyEvent (delegate Custom|SetPerceptionStateUI) 0.3 true))

(event EventTick
  (params (DeltaSeconds :type Float%20%28single-precision%29))
  (Variables|Default|SetLookingRotation (.yaw (Math|Rotator|FindLookatRotation (Math|Vector|MakeVector 0.0 0.0 0.0) (Variables|Default|GetTargetDirection))))
  (Default|LookatCamera (Variables|Default|GetFlipbookUpdateComponent) (Variables|Default|GetArrow) (Variables|Default|GetPaperFlipbook))
  (bind _anglenum (Default|GetAngleNumber (Variables|Default|GetFlipbookUpdateComponent) (Transformation|GetActorLocation self) (Variables|Default|GetLookingRotation) false))
  (bind _output_get (Variables|Default|SetAngleNum _anglenum))
  (Default|SetFlipbookbyAngleNum (Variables|Default|GetFlipbookUpdateComponent) (Variables|Default|GetCurrentAnimation) (Variables|Default|GetAngleNum) (Variables|Default|GetPaperFlipbook)) ; AngleNum과 Current Animation이 변할때만 실행되도록 개선할 것
  (Utilities|TargetDirectionDebug))

(event EventCauseDamage
  (params (BaseDamage :type Float%20%28single-precision%29) (PoiseDamage :type Float%20%28single-precision%29) (PushPower :type Float%20%28single-precision%29) (PushDirection :type Vector :default "0, 0, 0") (HitFromDirection :type Vector :default "0, 0, 0") (DamageCauser :type Actor%20Object%20Reference) (DamageInstigator :type Controller%20Object%20Reference))
  (|CallParentFunction BaseDamage PoiseDamage PushPower "0, 0, 0" "0, 0, 0" 0 0))

(fn ConstructionScript)