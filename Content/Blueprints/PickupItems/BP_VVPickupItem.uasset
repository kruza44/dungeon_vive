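; BP_VVPickupItem is a pickup item actor with a camera-facing sprite and an interaction text prompt.
; On BeginPlay it fills its UI_InteractText widget with the result of GetInteractText.
; Each Tick, FlipbookUpdateComponent turns the sprite toward the camera using the Arrow component.
; ShowInteractText and HideInteractText toggle the prompt widget's visibility and always return true.
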(event EventBeginPlay
  (bind _asui_interact_text (Utilities|Casting|CastToUI_InteractText (UserInterface|GetUserWidgetObject (Variables|Default|GetInteractTextWidget))))
  (Rendering|Components|TextRender|SetText (Variables|/Game/Blueprints/Widgets/UI_InteractText.UI_InteractText_C|GetInteractText _asui_interact_text) (Class|VVPickupItem|GetInteractText)))

(event EventTick
  (params (DeltaSeconds :type Float%20%28single-precision%29))
  (Default|LookatCamera (Variables|Default|GetFlipbookUpdateComponent) (Variables|Default|GetArrow) (Variables|Default|GetSprite)))

(fn ConstructionScript)

(fn ShowInteractText
  (Rendering|SetVisibility (Variables|Default|GetInteractTextWidget) true false)
  (return true))

(fn HideInteractText
  (Rendering|SetVisibility (Variables|Default|GetInteractTextWidget) false false)
  (return true))