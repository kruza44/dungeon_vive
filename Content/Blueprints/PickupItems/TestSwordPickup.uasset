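; Test sword pickup item that, when used from an inventory, equips a sword on the player.
; UseAction spawns a TestSword_BP, stores it as the player's HoldingWeapon and attaches it to the sprite's hand socket.
; It then calls the parent UseAction, commented as delete and destroy.
; Only ProtoPlayer_BP owners are supported; others just print a failure, with a TODO to generalize to Unit for enemies.
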(event EventBeginPlay
  (|CallParentFunction) ; This node is disabled and will not be called.\nDrag off pins to build functionality.
)

(event Collision|EventActorBeginOverlap
  (params (OtherActor :type Actor%20Object%20Reference)))

(event EventTick
  (params (DeltaSeconds :type Float%20%28single-precision%29))
  (|CallParentFunction DeltaSeconds) ; This node is disabled and will not be called.\nDrag off pins to build functionality.
)

(fn ConstructionScript
  (|CallParentFunction))

(fn UseAction
  (params (OwnerInventory :type Inventory%20Bag%20Object%20Reference) (InventoryIndex :type Integer))
  (bind _asproto_player_bp (Utilities|Casting|CastToProtoPlayer_BP (Variables|/Script/Vive.InventoryBag|GetOwnerUnit OwnerInventory)) ; TODO: 적들도 가능하게 하려면 Unit으로 일반화해야함
    (:then
      (bind _returnvalue (Game|SpawnActorfromClass "/Game/Blueprints/Weapons/TestSword_BP.TestSword_BP_C" (Transformation|GetSocketTransform (Variables|/Game/Blueprints/ProtoPlayer_BP.ProtoPlayer_BP_C|GetSprite _asproto_player_bp) "1_HandSocket" "RTS_World") "AlwaysSpawn" 0 0))
      (Variables|/Game/Blueprints/ProtoPlayer_BP.ProtoPlayer_BP_C|SetHoldingWeapon _asproto_player_bp _returnvalue)
      (Transformation|AttachComponentToComponent _returnvalue (Variables|/Game/Blueprints/ProtoPlayer_BP.ProtoPlayer_BP_C|GetSprite _asproto_player_bp) "1_HandSocket" "SnapToTarget" "SnapToTarget" "KeepWorld" true)
      (bind _returnvalue_2 (|CallParentFunction OwnerInventory InventoryIndex)) ; Delete and destroy
      (return _returnvalue_2))
    (:CastFailed
      (Development|PrintString "Sword cast failed"))))