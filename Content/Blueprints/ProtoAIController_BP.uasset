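; Prototype AI controller that starts behavior tree AI on the pawn it possesses.
; On possess it prints debug feedback on whether the pawn is a UnitPawn with an AIPerceptionComponent.
; It seeds the blackboard with the pawn's home position, PerceptionSphere component and a one-time copy of its perception state, then runs the behavior tree.
; An unconnected leftover graph would set TargetObject to the first perceived actor.
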(event EventPossess
  (params (PossessedPawn :type Pawn%20Object%20Reference))
  (bind _returnvalue (Actor|GetComponentbyClass PossessedPawn "/Script/Vive.PerceptionSphere"))
  (bind _blackboard (Variables|Default|GetBlackboard))
  (bind _asunit_pawn (Utilities|Casting|CastToUnitPawn PossessedPawn)
    (:then
      (Utilities|IsValid (Actor|GetComponentbyClass _asunit_pawn "/Script/AIModule.AIPerceptionComponent")
        (:Is%20Valid
          (Development|PrintString "Hello" true true "(R=0.361609,G=0.000000,B=1.000000,A=1.000000)"))
        (:Is%20Not%20Valid
          (Development|PrintString "Nello" true true "(R=1.000000,G=0.014252,B=0.000000,A=1.000000)" :!label _label))))
    (:CastFailed
      (goto _label)))
  (Utilities|FlowControl|Sequence
    (:then_0
      (Class|AIController|UseBlackboard)
      (AI|Components|Blackboard|SetValueasVector _blackboard (Variables|Default|GetHomePositionKey) (Transformation|GetActorLocation (Pawn|GetControlledPawn)))
      (AI|Components|Blackboard|SetValueasObject _blackboard (Utilities|Name|MakeLiteralName "PerceptionComp") _returnvalue)
      (AI|Components|Blackboard|SetValueasEnum _blackboard (Utilities|Name|MakeLiteralName "PerceptionState") (Variables|/Script/Vive.PerceptionSphere|GetPerceptionState _returnvalue)))
    (:then_1
      (AI|RunBehaviorTree))))

(fn ConstructionScript)