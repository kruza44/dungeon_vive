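; Prototype enemy Blueprint that reacts to hits and displays a perception test readout.
; Each tick it copies the perception sphere's test HUD string into its perception state widget, printing a message if the cast fails.
; Point damage writes push direction, a fixed push speed and a hit flag to the AI controller's blackboard.
; CauseDamage simply forwards base and poise damage to the parent class.
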(event EventBeginPlay
  ;[1 1 1] PerceptionStateTestUI
)

(event EventTick
  (params (DeltaSeconds :type Float%20%28single-precision%29))
  ;[1 1 1] PerceptionStateTestUI
  (bind _asperception_state_widget (Utilities|Casting|CastToPerceptionStateWidget (UserInterface|GetUserWidgetObject (Variables|Default|GetPerceptionStateWidget)))
    (:then
      (Variables|/Game/Blueprints/Widgets/PerceptionStateWidget.PerceptionStateWidget_C|SetPerceptionMeter _asperception_state_widget (Variables|/Script/Vive.PerceptionSphere|GetTestHUDString (Variables|Default|GetPerceptionSphere))))
    (:CastFailed
      (Development|PrintString "ProtoEnemeyWidgetCastFailed" true true "(R=1.000000,G=0.580944,B=0.000000,A=1.000000)"))))

(event EventCauseDamage
  (params (BaseDamage :type Float%20%28single-precision%29) (PoiseDamage :type Float%20%28single-precision%29) (PushPower :type Float%20%28single-precision%29) (PushDirection :type Vector :default "0, 0, 0") (HitFromDirection :type Vector :default "0, 0, 0") (DamageCauser :type Actor%20Object%20Reference) (DamageInstigator :type Controller%20Object%20Reference))
  (|CallParentFunction BaseDamage PoiseDamage 0.0 "0, 0, 0" "0, 0, 0" 0 0))

(event Game|Damage|EventPointDamage
  (params (Damage :type Float%20%28single-precision%29) (DamageType :type Damage%20Type%20Object%20Reference) (HitLocation :type Vector :default "0, 0, 0") (HitNormal :type Vector :default "0, 0, 0") (HitComponent :type Primitive%20Component%20Object%20Reference) (BoneName :type Name :default "None") (ShotFromDirection :type Vector :default "0, 0, 0") (InstigatedBy :type Controller%20Object%20Reference) (DamageCauser :type Actor%20Object%20Reference) (HitInfo :type Hit%20Result%20Structure%20%28by%20ref%29))
  (bind _returnvalue (Pawn|GetController))
  (bind _returnvalue_2 (AI|GetBlackboard _returnvalue))
  (AI|Components|Blackboard|SetValueasVector _returnvalue_2 (Utilities|Name|MakeLiteralName "PushedDirection") ShotFromDirection)
  (AI|Components|Blackboard|SetValueasFloat _returnvalue_2 (Utilities|Name|MakeLiteralName "PushedSpeed") 2e+02)
  (AI|Components|Blackboard|SetValueasBool _returnvalue_2 (Utilities|Name|MakeLiteralName "GotHitFlag") true))

(fn ConstructionScript)