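; BP_Spell is a base spell Blueprint that defines the shared interface for activating, casting and showing range UI for spells.
; Its events are empty, and UpdateSpellPositionUI and IsCasting return placeholder values, apparently for child spells to override.
; Getters expose the max and spell radii, whether each needs range UI, and the casting-finished state, which ResetSpellVariables clears along with the timer.
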(event Custom|CastSpell)

(event Custom|ActivateSpell)

(event Custom|ShowSpellRangeUI)

(event Custom|HideSpellRangeUI)

(event Custom|CastingFailed)

(fn ConstructionScript)

(fn IsNeedMaxRangeUI
  (return (Variables|Default|GetbNeedMaxRangeUI)))

(fn IsNeedSpellRangeUI
  (return (Variables|Default|GetbNeedSpellRangeUI)))

(fn GetMaxRadius
  (return (Variables|Default|GetMaxRadius)))

(fn GetSpellRadius
  (return (Variables|Default|GetSpellRadius)))

(fn UpdateSpellPositionUI
  (params (MoveDirection :type Vector))
  (return "0, 0, 0"))

(fn IsCastingFinished
  (return (Variables|Default|GetbIsCastingFinished)))

(fn ResetSpellVariables
  (Variables|Default|SetbIsCastingFinished false)
  (Variables|Default|SetTimer 0.0))

(fn IsCasting
  (return false))