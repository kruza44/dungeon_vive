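; BP_SpellRangeUI is an actor that visualizes a spell's range with a decal.
; SetRadius scales the decal's Y and Z axes by the radius divided by its DecalSize Y, and the construction script applies it from the Radius variable.
; ShowSpellRange and HideSpellRange toggle the actor's visibility in game, and the event graph holds no active logic.
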(event EventBeginPlay)

(event Collision|EventActorBeginOverlap
  (params (OtherActor :type Actor%20Object%20Reference)))

(event EventTick
  (params (DeltaSeconds :type Float%20%28single-precision%29)))

(fn ConstructionScript
  (CallFunction|SetRadius (Variables|Default|GetRadius)))

(fn SetRadius
  (params (Radius :type Float%20%28single-precision%29))
  (bind _decal (Variables|Default|GetDecal))
  (bind _decalsize (Variables|/Script/Engine.DecalComponent|GetDecalSize _decal))
  (bind _returnvalue (/ Radius (.y _decalsize)))
  (Transformation|SetWorldScale3D (Variables|Default|GetDecal) (Math|Vector|MakeVector 1.0 _returnvalue _returnvalue)))

(fn ShowSpellRange
  (Rendering|SetActorHiddenInGame false))

(fn HideSpellRange
  (Rendering|SetActorHiddenInGame true))