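; Fireball spell Blueprint that lets the caster aim an explosion area, then charges and launches a projectile at it.
; Two spawned, reused range indicators show maximum range and blast radius; target movement slides along a hardcoded distance limit via plane projection.
; CastSpell accumulates time, spawning SE_FireballProjectile above the owner after one second and launching it at CastingTime.
; A failed cast enables gravity on any spawned fireball, dropping it.
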(event EventCastingFailed
  ;[1 1 1] Cast spell and finish
  (bind _fireballprojectile (Variables|Default|GetFireballProjectile)
    (:then
      (Default|EnableGravity _fireballprojectile) ; When failed casting, drop fireball
    )
    (:else)))

(event EventResetSpellVariables
  ;[1 1 1] Cast spell and finish
  (|CallParentFunction)
  (Variables|Default|SetbFireballSpawned false))

(event EventCastSpell
  (bind _returnvalue (Components|GetOwner))
  ;[1 1 1] Cast spell and finish
  (bind _output_get (Variables|Default|SetTimer (+ (Variables|Default|GetTimer) (Utilities|Time|GetWorldDeltaSeconds))))
  (if (>= _output_get 1.0) ; Spawn fireball at 2sec
    (if (Variables|Default|GetbFireballSpawned)
      _
      (else
        (bind _returnvalue_2 (Game|SpawnActorfromClass "/Game/Blueprints/Spells/SpellEffects/SE_FireballProjectile.SE_FireballProjectile_C" (Math|Transform|MakeTransform (+ "0, 0,10.000000" (Transformation|GetActorLocation _returnvalue)) "0, 0, 0" "1,1,1") "Undefined" _returnvalue (Variables|Default|GetTargetPosition) (Variables|Default|GetSpellRadius) 0))
        (Variables|Default|SetbFireballSpawned true)
        (bind _output_get_2 (Variables|Default|SetFireballProjectile _returnvalue_2))))
    (if (>= (Variables|Default|GetTimer) (Variables|Default|GetCastingTime)) ; Casting Finished
      (Variables|Default|SetbIsCastingFinished true)
      (Default|LaunchProjectile _output_get_2))))

(event EventActivateSpell)

(event EventBeginPlay
  (Variables|Default|SetTimer 0.0))

(event EventTick
  (params (DeltaSeconds :type Float%20%28single-precision%29)))

(event EventShowSpellRangeUI
  (bind _returnvalue (Components|GetOwner))
  (bind _returnvalue_2 (Transformation|GetActorLocation _returnvalue))
  ;[1 1 1] Hide and show spell range UI
  (bind _maxspellrangeui (Variables|Default|GetMaxSpellRangeUI)
    (:then
      (Transformation|SetActorLocation _maxspellrangeui _returnvalue_2 false false)
      (Default|ShowSpellRange _maxspellrangeui))
    (:else
      (bind _returnvalue_3 (Game|SpawnActorfromClass "/Game/Blueprints/Spells/BP_SpellRangeUI.BP_SpellRangeUI_C" (Math|Transform|MakeTransform _returnvalue_2 "0, 0, 0" "1,1,1") "Undefined" self (Variables|Default|GetMaxRadius) 0))
      (Variables|Default|SetMaxSpellRangeUI _returnvalue_3)))
  (bind _output_get (Variables|Default|SetTargetPosition (Transformation|GetActorLocation (Components|GetOwner))))
  (bind _spelleffectrangeui (Variables|Default|GetSpellEffectRangeUI)
    (:then
      (Transformation|SetActorLocation _spelleffectrangeui _output_get false false)
      (Default|ShowSpellRange _spelleffectrangeui))
    (:else
      (bind _returnvalue_4 (Game|SpawnActorfromClass "/Game/Blueprints/Spells/BP_SpellRangeUI.BP_SpellRangeUI_C" (Math|Transform|MakeTransform _output_get "0, 0, 0" "1,1,1") "Undefined" self (Variables|Default|GetSpellRadius) 0))
      (Variables|Default|SetSpellEffectRangeUI _returnvalue_4))))

(event EventHideSpellRangeUI
  ;[1 1 1] Hide and show spell range UI
  (Default|HideSpellRange (Variables|Default|GetMaxSpellRangeUI))
  (Default|HideSpellRange (Variables|Default|GetSpellEffectRangeUI)))

(fn ConstructionScript
  (|CallParentFunction))

(fn UpdateSpellPositionUI
  (params (MoveDirection :type Vector :default "0, 0, 0"))
  (bind _spelleffectrangeui (Variables|Default|GetSpellEffectRangeUI))
  (if (and (>= (Math|Vector|VectorLength (- (Transformation|GetActorLocation (Components|GetOwner)) (Variables|Default|GetTargetPosition))) 3e+02) (< (Math|Vector2D|DotProduct(2D) (Math|Vector2D|MakeVector2D (.x (- (Transformation|GetActorLocation (Components|GetOwner)) (Variables|Default|GetTargetPosition))) (.y (- (Transformation|GetActorLocation (Components|GetOwner)) (Variables|Default|GetTargetPosition)))) (Math|Vector2D|MakeVector2D (.x MoveDirection) (.y MoveDirection))) 0.0))
    (bind _output_get (Variables|Default|SetTargetPosition (+ (Variables|Default|GetTargetPosition) (Math|Vector|ProjectVectorontoPlane (* MoveDirection 5.0) (Math|Vector|Normalize (- (Transformation|GetActorLocation (Components|GetOwner)) (Variables|Default|GetTargetPosition)))))))
    (Transformation|SetActorLocation _spelleffectrangeui _output_get false false)
    (else
      (bind _output_get_2 (Variables|Default|SetTargetPosition (+ (Variables|Default|GetTargetPosition) (* MoveDirection 3.0))))
      (Transformation|SetActorLocation _spelleffectrangeui _output_get_2 false false)))
  (return (Variables|Default|GetTargetPosition)))