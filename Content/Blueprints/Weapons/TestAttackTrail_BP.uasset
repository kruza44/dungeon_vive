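; Test Blueprint for previewing weapon attack trails: DoAttack plays an animation on a skeletal mesh and starts particle trails between two sockets.
; It also spawns the same particle template attached at the first socket.
; A timeline matched to the animation's length and play rate sets trail lifetime from a swappable curve or a constant.
; When the timeline finishes with looping enabled, it waits, then stops the mesh and ends the trails.
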(event EventBeginPlay
  (Effects|Components|ParticleSystem|SetTemplate (Variables|Default|GetTrailParticle) (Variables|Default|GetParticleVar)))

(event EventDoAttack
  (bind _timeline_0 (Variables|Default|GetTimeline_0))
  (bind _playrate (Variables|Default|GetPlayRate))
  (bind _trailparticle (Variables|Default|GetTrailParticle))
  (bind _lifetimename (Variables|Default|GetLifeTimeName))
  (bind _skeletalmesh (Variables|Default|GetSkeletalMesh))
  (Components|Animation|SetPosition (Variables|Default|GetSkeletalMesh) 0.0 false)
  (Components|Timeline|SetPlayRate (Variables|Default|GetSkeletalMesh) (Variables|Default|GetPlayRate))
  (bind _returnvalue (Animation|GetPlayLength (Variables|Default|GetAnimVar)))
  (Variables|Default|SetTimeVar _returnvalue)
  (Effects|SpawnEmitterAttached (Variables|Default|GetParticleVar) _skeletalmesh (Variables|Default|GetFirstSocketName) (Variables|/Script/Engine.SceneComponent|GetRelativeLocation _skeletalmesh) "-90.000000, 0, 0")
  (Effects|Particles|Trails|BeginTrails (Variables|Default|GetTrailParticle) (Variables|Default|GetFirstSocketName) (Variables|Default|GetSecondSocketName) "ETrailWidthMode_FromCentre" 1.0)
  (Components|Animation|PlayAnimation (Variables|Default|GetSkeletalMesh) (Variables|Default|GetAnimVar) (Variables|Default|GetIsLooping))
  (Components|Timeline|SetTimelineLength _timeline_0 (Variables|Default|GetTimeVar))
  (Components|Timeline|SetPlayRate (Variables|Default|GetSkeletalMesh) _playrate)
  (Components|Timeline|SetPlayRate _timeline_0 _playrate)
  (Class|TimelineComponent|SetFloatCurve (Variables|Default|GetTimeline_0) (Variables|Default|GetCurveVar) "Discount")
  (bind _discount (Timeline|Timeline_0 PlayFromStart)
    (:Update
      (if (Variables|Default|GetIsTimeline) ; TimeLine or Constant
        (Effects|Components|ParticleSystem|SetFloatParameter _trailparticle _lifetimename _discount)
        (else
          (Effects|Components|ParticleSystem|SetFloatParameter _trailparticle _lifetimename (Variables|Default|GetTrailLifeTime)))))
    (:Finished
      (if (not (not (Variables|Default|GetIsLooping)))
        (Utilities|FlowControl|Delay (Variables|Default|GetDelayTime))
        (Audio|Components|Audio|Stop (Variables|Default|GetSkeletalMesh))
        (Effects|Particles|Trails|EndTrails (Variables|Default|GetTrailParticle))
        (Development|PrintString "TrailFinishied" true true "(R=0.000000,G=1.000000,B=0.213846,A=1.000000)")))))

(fn ConstructionScript)