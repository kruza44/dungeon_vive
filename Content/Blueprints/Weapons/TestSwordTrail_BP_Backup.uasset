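; Test sword actor that plays an attack animation with a particle weapon trail between two mesh sockets.
; DoAttack starts the trail and a timeline matched to animation length, driving trail lifetime from a curve or constant, restarting after a delay when looping.
; BeginPlay sets the trail template and loads weapon data from a DataTable.
; Hitbox overlap, marked deprecated, applies point damage from that data if the attach parent has a UnitStat_BP.
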(event OnComponentBeginOverlap(HitBox)
  (params (OverlappedComponent :type Primitive%20Component%20Object%20Reference) (OtherActor :type Actor%20Object%20Reference) (OtherComp :type Primitive%20Component%20Object%20Reference) (OtherBodyIndex :type Integer) (bFromSweep :type Boolean) (SweepResult :type Hit%20Result%20Structure%20%28by%20ref%29))
  (bind _returnvalue (Actor|GetAttachParentActor))
  (bind _returnvalue_2 (Transformation|GetActorLocation OtherActor))
  (bind _weapondata (Variables|Default|GetWeaponData))
  (bind _basedamage (Utilities|Struct|BreakWeaponData _weapondata))
  (bind _returnvalue_3 (Transformation|GetActorLocation _returnvalue))
  (bind _returnvalue_4 (- _returnvalue_2 _returnvalue_3))
  (bind _returnvalue_5 (+ 5.0 _basedamage))
  ;[1 1 1] 폐기
  (Utilities|IsValid (Actor|GetComponentbyClass _returnvalue "/Game/Blueprints/UnitStat_BP.UnitStat_BP_C")
    (:Is%20Valid
      (Development|PrintString (Utilities|String|ToString(Float) _returnvalue_5) true true "(R=0.000000,G=0.114498,B=1.000000,A=1.000000)")
      (Game|Damage|ApplyPointDamage OtherActor _returnvalue_5 (Math|Vector|Normalize (Math|Vector|MakeVector (.x _returnvalue_4) (.y _returnvalue_4) 0.0)) SweepResult 0 _returnvalue))
    (:Is%20Not%20Valid
      (Development|PrintString "TestSwordTrail_BP UnitStat_BP Is NOT VALID" true true "(R=1.000000,G=0.000000,B=0.071409,A=1.000000)"))))

(event Custom|DoAttack
  (bind _timeline_0 (Variables|Default|GetTimeline_0))
  (bind _playrate (Variables|Default|GetPlayRate))
  (bind _particle_trail (Variables|Default|GetParticle_Trail))
  (bind _lifetimename (Variables|Default|GetLifeTimeName))
  (bind _skeletalmesh (Variables|Default|GetSkeletalMesh))
  (Components|Animation|SetPosition (Variables|Default|GetSkeletalMesh) 0.0 false :!label _label)
  (Components|Timeline|SetPlayRate (Variables|Default|GetSkeletalMesh) (Variables|Default|GetPlayRate))
  (bind _returnvalue (Animation|GetPlayLength (Variables|Default|GetAnimVar)))
  (Variables|Default|SetTimeVar _returnvalue)
  (Effects|SpawnEmitterAttached (Variables|Default|GetParticleVar) _skeletalmesh (Variables|Default|GetFirstSocketName) (Variables|/Script/Engine.SceneComponent|GetRelativeLocation _skeletalmesh) "-90.000000, 0, 0")
  (Effects|Particles|Trails|BeginTrails (Variables|Default|GetParticle_Trail) (Variables|Default|GetFirstSocketName) (Variables|Default|GetSecondSocketName_0) "ETrailWidthMode_FromCentre" 1.0)
  (Components|Animation|PlayAnimation (Variables|Default|GetSkeletalMesh) (Variables|Default|GetAnimVar) (Variables|Default|GetIsLooping))
  (Components|Timeline|SetTimelineLength _timeline_0 (Variables|Default|GetTimeVar))
  (Components|Timeline|SetPlayRate (Variables|Default|GetSkeletalMesh) _playrate)
  (Components|Timeline|SetPlayRate _timeline_0 _playrate)
  (Class|TimelineComponent|SetFloatCurve (Variables|Default|GetTimeline_0) (Variables|Default|GetCurveVar) "discount")
  (bind _discount (Timeline|Timeline_0 PlayFromStart)
    (:Update
      (if (Variables|Default|GetIsTimeline) ; TimeLine or Constant
        (Effects|Components|ParticleSystem|SetFloatParameter _particle_trail _lifetimename _discount)
        (else
          (Effects|Components|ParticleSystem|SetFloatParameter _particle_trail _lifetimename (Variables|Default|GetTrailLifeTime)))))
    (:Finished
      (if (not (not (Variables|Default|GetIsLooping)))
        (Utilities|FlowControl|Delay (Variables|Default|GetDelayTime))
        (Audio|Components|Audio|Stop (Variables|Default|GetSkeletalMesh))
        (Effects|Particles|Trails|EndTrails (Variables|Default|GetParticle_Trail))
        (goto _label)))))

(event EventBeginPlay
  (Effects|Components|ParticleSystem|SetTemplate (Variables|Default|GetParticle_Trail) (Variables|Default|GetParticleVar))
  (bind _returnvalue (Utilities|GetDataTableRow "/Game/Data/Weapons.Weapons" (.RowName (Utilities|Struct|BreakDataTableRowHandle (Variables|Default|GetWeaponInDataTable))))
    (:then
      (bind _output_get (Variables|Default|SetWeaponData _returnvalue)))))

(fn ConstructionScript)