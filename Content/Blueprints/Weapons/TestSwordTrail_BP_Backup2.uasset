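; Test Blueprint for previewing a sword swing animation with a particle weapon trail between two sockets.
; DoAttack plays the animation on the skeletal mesh, spawns an attached emitter and begins trails on the particle component.
; A timeline matched to animation length and play rate drives trail lifetime from a curve or constant.
; When looping, it stops animation and trail after a delay once the timeline finishes; the weapon DataTable lookup is unconnected.
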(event Custom|DoAttack
  (bind _timeline_0 (Variables|Default|GetTimeline_0))
  (bind _playrate (Variables|Default|GetPlayRate))
  (bind _particle_trail (Variables|Default|GetParticle_Trail))
  (bind _lifetimename (Variables|Default|GetLifeTimeName))
  (bind _skeletalmesh (Variables|Default|GetSkeletalMesh))
  (Components|Animation|SetPosition (Variables|Default|GetSkeletalMesh) 0.0 false)
  (Components|Timeline|SetPlayRate (Variables|Default|GetSkeletalMesh) (Variables|Default|GetPlayRate))
  (bind _returnvalue (Animation|GetPlayLength (Variables|Default|GetAnimVar)))
  (Variables|Default|SetTimeVar _returnvalue)
  (Effects|SpawnEmitterAttached (Variables|Default|GetParticleVar) _skeletalmesh (Variables|Default|GetFirstSocketName) (Variables|/Script/Engine.SceneComponent|GetRelativeLocation _skeletalmesh) "-90.000000, 0, 0")
  (Effects|Particles|Trails|BeginTrails (Variables|Default|GetParticle_Trail) (Variables|Default|GetFirstSocketName) (Variables|Default|GetSecondSocketName_0) "ETrailWidthMode_FromCentre" 1.0)
  (Components|Animation|PlayAnimation (Variables|Default|GetSkeletalMesh) (Variables|Default|GetAnimVar) (Variables|Default|GetIsLooping))
  (Components|Timeline|SetTimelineLength _timeline_0 (Variables|Default|GetTimeVar))
  (Components|Timeline|SetPlayRate (Variables|Default|GetSkeletalMesh) _playrate)
  (Components|Timeline|SetPlayRate _timeline_0 _playrate)
  (Class|TimelineComponent|SetFloatCurve (Variables|Default|GetTimeline_0) (Variables|Default|GetCurveVar) "discount")
  (bind _discount (Timeline|Timeline_0 PlayFromStart)
    (:Update
      (if (Variables|Default|GetIsTimeline) ; TimeLine or Constant
        (Effects|Components|ParticleSystem|SetFloatParameter _particle_trail _lifetimename _discount)
        (else
          (Effects|Components|ParticleSystem|SetFloatParameter _particle_trail _lifetimename (Variables|Default|GetTrailLifeTime)))))
    (:Finished
      (if (not (not (Variables|Default|GetIsLooping)))
        (Utilities|FlowControl|Delay (Variables|Default|GetDelayTime))
        (Audio|Components|Audio|Stop (Variables|Default|GetSkeletalMesh))
        (Effects|Particles|Trails|EndTrails (Variables|Default|GetParticle_Trail))))))

(event EventBeginPlay
  (Effects|Components|ParticleSystem|SetTemplate (Variables|Default|GetParticle_Trail) (Variables|Default|GetParticleVar)))

(fn ConstructionScript)