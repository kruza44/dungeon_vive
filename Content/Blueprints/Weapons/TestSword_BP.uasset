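; TestSword_BP is a test sword weapon that draws its data and flipbook sprite from the Weapons data table.
; On BeginPlay it looks up its configured row, stores it as WeaponData and applies the first sprite to WeaponSprite.
; StartAttack and EndAttack toggle the attack flag, and EndAttack also clears the HitActors list; no hit detection is implemented here.
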(event Custom|TestEvent)

(event EventBeginPlay
  (bind _returnvalue (Utilities|GetDataTableRow "/Game/Data/Weapons.Weapons" (.RowName (Utilities|Struct|BreakDataTableRowHandle (Variables|Default|GetWeaponInDataTable))))
    (:then
      (bind _output_get (Variables|Default|SetWeaponData _returnvalue))
      (Sprite|SetFlipbook (Variables|Default|GetWeaponSprite) (Utilities|Array|Get(acopy) (.Sprites (Utilities|Struct|BreakWeaponData _output_get)))))))

(fn ConstructionScript)

(fn StartAttack
  (Variables|Default|SetIsInAttack true))

(fn EndAttack
  (Variables|Default|SetIsInAttack false)
  (Utilities|Array|Clear (Variables|Default|GetHitActors)))